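; First-person HUD Blueprint that creates the main HUD widget and opens and closes the shop panel.
; A custom event adds WBP_HUDWidget to the viewport.
; ShowShop adds WBP_ShopPanel, stops character movement, switches the player controller to the shop input context and enables cursor-driven Game and UI input.
; CloseShop removes the cached panel and restores the main player context and game-only input.
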(event EventCreateHUDWidget
  (bind _returnvalue (UserInterface|CreateWidget "/Game/FPSGAME/Blueprint/UI/WBP_HUDWidget.WBP_HUDWidget_C" (Game|GetPlayerController 0)))
  (Utilities|IsValid _returnvalue
    (:Is%20Valid
      (UserInterface|Viewport|AddtoViewport _returnvalue 0))))

(fn ConstructionScript)

(fn ShowShop
  (bind _asbp_fp_player_controller (Utilities|Casting|CastToBP_FP_PlayerController (Game|GetPlayerController 0)))
  (Utilities|IsValid _asbp_fp_player_controller
    (:Is%20Valid
      (Variables|Default|SetPlayerContollerRef _asbp_fp_player_controller)
      (bind _returnvalue (UserInterface|CreateWidget "/Game/FPSGAME/Blueprint/UI/Shop/WBP_ShopPanel.WBP_ShopPanel_C" (Variables|Default|GetPlayerContollerRef)))
      (bind _output_get (Variables|Default|SetWBPShopPanelRef _returnvalue))
      (UserInterface|Viewport|AddtoViewport _output_get 0)
      (Components|Movement|StopMovementImmediately (Variables|/Script/Engine.Character|GetCharacterMovement (Game|GetPlayerCharacter 0)))
      (Class|FPPlayerController|SwitchContext (Variables|Default|GetPlayerContollerRef) "/Game/FPSGAME/Input/Shop/IMC_Shop.IMC_Shop")
      (Input|SetInputModeGameandUI (Variables|Default|GetPlayerContollerRef) 0 "DoNotLock" false false)
      (Variables|/Script/Engine.PlayerController|SetbShowMouseCursor (Variables|Default|GetPlayerContollerRef) true))))

(fn CloseShop
  (bind _playercontollerref (Variables|Default|GetPlayerContollerRef))
  (bind _wbpshoppanelref (Variables|Default|GetWBPShopPanelRef)
    (:then
      (Widget|RemovefromParent _wbpshoppanelref)
      (Class|FPPlayerController|SwitchContext _playercontollerref "/Game/FPSGAME/Input/IMC_MainPlayer.IMC_MainPlayer")
      (Input|SetInputModeGameOnly _playercontollerref false)
      (Variables|/Script/Engine.PlayerController|SetbShowMouseCursor _playercontollerref false))
    (:else)))