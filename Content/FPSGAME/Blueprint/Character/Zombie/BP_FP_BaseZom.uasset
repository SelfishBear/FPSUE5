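; BP_FP_BaseZom is the base zombie enemy, providing its melee hit check and death handling.
; On health component death, it disables capsule collision and sends a Death event to its StateTree AI.
; TryHitPlayer sphere-traces forward using the current attack's distance and radius, applying damage through the FP_Damageable interface, with persistent debug drawing left on.
; FinishDeath destroys the actor as a separate step.
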(event OnDeath(FP_HealthComponent)
  (Collision|SetCollisionEnabled (Variables|Default|GetCapsuleComponent) "NoCollision")
  (Gameplay|StateTree|SendStateTreeEvent (Variables|Default|GetStateTreeAI) (Utilities|Struct|MakeStateTreeEvent "(TagName=\"Death\")" "None" "None") :!class /Script/GameplayStateTreeModule.StateTreeComponent))

(fn ConstructionScript)

(fn TryHitPlayer
  (bind _returnvalue (Transformation|GetActorLocation))
  (bind _returnvalue_2 (+ (.z _returnvalue) 25.0))
  (bind _returnvalue_3 (Math|Vector|MakeVector (.x _returnvalue) (.y _returnvalue) _returnvalue_2))
  (bind _outhit (Collision|SphereTraceByChannel _returnvalue_3 (+ _returnvalue_3 (* (Transformation|GetActorForwardVector) (Variables|Default|GetCurrentAttackTraceDistance))) (Variables|Default|GetCurrentAttackRadius) "TraceTypeQuery3" false 0 "Persistent"))
  (if (Utilities|DoesObjectImplementInterface (.hitactor _outhit) "/Script/FPSGame.FP_Damageable")
    (bind _asfp_damageable (Utilities|Casting|CastToFP_Damageable (.hitactor _outhit)))
    (Class|FPDamageable|ReceiveDamage _asfp_damageable (Variables|Default|GetCurrentAttackDamage))))

(fn FinishDeath
  (Actor|DestroyActor))