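; Base zombie enemy that takes damage, dies and performs melee attacks.
; Incoming damage goes to its FPHealth component; on death it disables capsule collision and sends a Death event to its StateTree.
; TryHitPlayer sphere-traces forward and damages a hit actor implementing FP_Damageable, while FinishDeath destroys the zombie.
; Debug output remains active: a health print on damage and persistent trace drawing.
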(event OnDeath(FP_Health)
  (params (bIsDead :type Boolean))
  (Collision|SetCollisionEnabled (Variables|Collision|GetCapsuleComponent) "NoCollision")
  (Gameplay|StateTree|SendStateTreeEvent (Variables|Default|GetStateTree) (Utilities|Struct|MakeStateTreeEvent "(TagName=\"Death\")" "None" "None") :!class /Script/GameplayStateTreeModule.StateTreeComponent))

(event EventDamage
  (params (DamageAmount :type Float%20%28single-precision%29))
  (Class|FPHealthComponent|TakeDamage (Variables|Default|GetFP_Health) DamageAmount)
  (Development|PrintString (Utilities|String|Append "Current Health" "-" (Utilities|String|ToString(Float) (Variables|/Script/FPSGame.FP_HealthComponent|GetCurrentHealth (Variables|Default|GetFP_Health))))))

(fn ConstructionScript)

(fn TryHitPlayer
  (bind _returnvalue (Transformation|GetActorLocation))
  (bind _returnvalue_2 (+ (.z _returnvalue) 25.0))
  (bind _returnvalue_3 (Math|Vector|MakeVector (.x _returnvalue) (.y _returnvalue) _returnvalue_2))
  (bind _outhit (Collision|SphereTraceByChannel _returnvalue_3 (+ _returnvalue_3 (* (Transformation|GetActorForwardVector) (Variables|Default|GetAttackTraceDistance))) (Variables|Default|GetAttackRadius) "TraceTypeQuery1" false 0 "Persistent"))
  (if (Utilities|DoesObjectImplementInterface (.hitactor _outhit) "/Script/FPSGame.FP_Damageable")
    (bind _asfp_damageable (Utilities|Casting|CastToFP_Damageable (.hitactor _outhit)))
    (Class|FPDamageable|ReceiveDamage _asfp_damageable (Variables|Default|GetDamage))))

(fn FinishDeath
  (Actor|DestroyActor))