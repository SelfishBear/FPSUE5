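; BP_ShopMerchant is a shop merchant actor that opens the shop UI when the first-person character overlaps its trigger.
; The ShopTrigger overlap confirms the other actor is BP_FP_Character, then calls ShowShop on player 0's BP_FP_HUD.
; PlayFeedback then plays a random sound from SoundWaves at the merchant's location, using the SA_Merchant attenuation settings.
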(event OnComponentBeginOverlap(ShopTrigger)
  (params (OverlappedComponent :type Primitive%20Component%20Object%20Reference) (OtherActor :type Actor%20Object%20Reference) (OtherComp :type Primitive%20Component%20Object%20Reference) (OtherBodyIndex :type Integer) (bFromSweep :type Boolean) (SweepResult :type Hit%20Result%20Structure%20%28by%20ref%29))
  (Utilities|Casting|CastToBP_FP_Character OtherActor)
  (bind _asbp_fp_hud (Utilities|Casting|CastToBP_FP_HUD (HUD|GetHUD (Game|GetPlayerController 0))))
  (Default|ShowShop _asbp_fp_hud)
  (CallFunction|PlayFeedback))

(fn ConstructionScript)

(fn PlayFeedback
  (Audio|PlaySoundatLocation (.OutItem (Utilities|Array|Random (Variables|Default|GetSoundWaves))) (Transformation|GetActorLocation) "0, 0, 0" 1.0 1.0 0.0 "/Game/FPSGAME/Sounds/ShopMerchant/SA_Merchant.SA_Merchant" 0 0 0))